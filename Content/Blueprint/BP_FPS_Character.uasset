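; First-person shooter player character Blueprint that handles movement, camera look, jumping, dashing and weapon input.
; Input axes drive capsule-relative movement and controller yaw and pitch.
; Dash launches the character forward, then briefly after upward, with a DoOnce and delay acting as cooldown.
; Mouse and key presses forward fire, reload and pickup to InventoryManager, while a Data Table walk-speed lookup sits unconnected.
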(event EventBeginPlay)

(event Collision|EventActorBeginOverlap
  (params (OtherActor :type Actor%20Object%20Reference)))

(event EventTick
  (params (DeltaSeconds :type Float%20%28single-precision%29)))

(event Input|ActionEvents|InputActionJump
  (params (Key :type Key%20Structure :default "None"))
  ;[0.15 0.15 0.15 0.5] Action Mappings
  (:Pressed
    (Character|Jump)))

(event Input|ActionEvents|InputActionDash
  (params (Key :type Key%20Structure :default "None"))
  (bind _returnvalue (Transformation|GetActorRotation))
  ;[0.15 0.15 0.15 0.5] Dash
  (:Pressed
    (Utilities|FlowControl|DoOnce false :!label _label
      (:Completed
        (Character|LaunchCharacter (* (Math|Vector|GetForwardVector _returnvalue) 8e+02) false false)
        (Utilities|FlowControl|Delay 0.01)
        (Character|LaunchCharacter (* (Math|Vector|GetUpVector _returnvalue) 2e+02) false false)
        (Utilities|FlowControl|Delay 1.0)
        (goto _label Reset)))))

(event Input|AxisEvents|InputAxisTurn
  (params (AxisValue :type Float%20%28single-precision%29))
  ;[0.15 0.15 0.15 0.5] Camera
  (Pawn|Input|AddControllerYawInput AxisValue))

(event Input|AxisEvents|InputAxisLookUp
  (params (AxisValue :type Float%20%28single-precision%29))
  ;[0.15 0.15 0.15 0.5] Camera
  (Pawn|Input|AddControllerPitchInput AxisValue))

(event Input|AxisEvents|InputAxisMoveForward
  (params (AxisValue :type Float%20%28single-precision%29))
  ;[0.15 0.15 0.15 0.5] Movement
  (Pawn|Input|AddMovementInput (Math|Vector|GetForwardVector (Variables|Collision|GetCapsuleComponent)) AxisValue false))

(event Input|AxisEvents|InputAxisMoveRight
  (params (AxisValue :type Float%20%28single-precision%29))
  ;[0.15 0.15 0.15 0.5] Movement
  (Pawn|Input|AddMovementInput (Math|Vector|GetRightVector (Variables|Collision|GetCapsuleComponent)) AxisValue false))

(event Input|KeyboardEvents|DebugKeyH
  (params (Key :type Key%20Structure :default "None") (ActionValue :type Input%20Action%20Value%20Structure))
  ;[0.15 0.15 0.15 0.5] How to make Data Table Connection
)

(event Input|KeyboardEvents|E
  (params (Key :type Key%20Structure :default "None"))
  (:Pressed
    (Class|InventoryManager|PickUpWeapon (Variables|Default|GetInventoryManager))))

(event Input|MouseEvents|LeftMouseButton
  (params (Key :type Key%20Structure :default "None"))
  (:Pressed
    (Class|InventoryManager|FireCurrentWeapon (Variables|Default|GetInventoryManager))))

(event Input|KeyboardEvents|R
  (params (Key :type Key%20Structure :default "None"))
  (:Pressed
    (Class|InventoryManager|ReloadCurrentWeapon (Variables|Default|GetInventoryManager))))

(fn ConstructionScript)